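; BP_Button is an interactable button that toggles a referenced actor between two positions.
; Its Box overlap events enable and disable player input and set IsOverlapped, so Use only works in range.
; Each press teleports Object by VectorOut or its inverse VectorIn, computed on BeginPlay, depending on IsActivated, which then flips.
; The button material turns green on press and red on release.
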(event OnComponentBeginOverlap(Box)
  (params (OverlappedComponent :type Primitive%20Component%20Object%20Reference) (OtherActor :type Actor%20Object%20Reference) (OtherComp :type Primitive%20Component%20Object%20Reference) (OtherBodyIndex :type Integer) (bFromSweep :type Boolean) (SweepResult :type Hit%20Result%20Structure%20%28by%20ref%29))
  ;[1 1 1] Range
  (Variables|Default|SetIs%20Overlapped true)
  (Input|EnableInput (Game|GetPlayerController 0)))

(event OnComponentEndOverlap(Box)
  (params (OverlappedComponent :type Primitive%20Component%20Object%20Reference) (OtherActor :type Actor%20Object%20Reference) (OtherComp :type Primitive%20Component%20Object%20Reference) (OtherBodyIndex :type Integer))
  ;[1 1 1] Range
  (Variables|Default|SetIs%20Overlapped false)
  (Input|DisableInput (Game|GetPlayerController 0)))

(event EventBeginPlay
  (Variables|Default|SetVectorIn (- (Variables|Default|GetVectorOut) (* (Variables|Default|GetVectorOut) 2.0))))

(event Input|ActionEvents|InputActionUse
  (params (Key :type Key%20Structure :default "None"))
  (:Pressed
    (if (Variables|Default|GetIs%20Overlapped)
      (Rendering|Material|SetMaterial (Variables|Default|GetButton) 0 "/Game/_MY_CONTENT_/Materials/M_Green.M_Green")
      (if (Variables|Default|GetIs%20Activated)
        (Transformation|SetActorLocation (Variables|Default|GetObject) (+ (Transformation|GetActorLocation (Variables|Default|GetObject)) (Variables|Default|GetVectorOut)) false true)
        (Variables|Default|SetIs%20Activated false)
        (else
          (Transformation|SetActorLocation (Variables|Default|GetObject) (+ (Transformation|GetActorLocation (Variables|Default|GetObject)) (Variables|Default|GetVectorIn)) false true)
          (Variables|Default|SetIs%20Activated true)))))
  (:Released
    (if (Variables|Default|GetIs%20Overlapped)
      (Rendering|Material|SetMaterial (Variables|Default|GetButton) 0 "/Game/_MY_CONTENT_/Materials/M_Red.M_Red"))))

(fn ConstructionScript)