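; BP_LobbyDoor is a lobby doorway that teleports the player to a level's location.
; On box overlap it moves MyPlayer to the TeleportLocation actor's position and plays a 2D teleport sound, without checking which actor overlapped.
; The construction script applies a blue hex-tile material to the cube and sets the title text from the Level variable.
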(event OnComponentBeginOverlap(Box)
  (params (OverlappedComponent :type Primitive%20Component%20Object%20Reference) (OtherActor :type Actor%20Object%20Reference) (OtherComp :type Primitive%20Component%20Object%20Reference) (OtherBodyIndex :type Integer) (bFromSweep :type Boolean) (SweepResult :type Hit%20Result%20Structure%20%28by%20ref%29))
  (Transformation|SetActorLocationAndRotation (Variables|Default|GetMy%20Player) (Transformation|GetActorLocation (Variables|Default|GetTeleport%20Location)) "0, 0, 0" false true)
  (Audio|PlaySound2D "/Game/_MY_CONTENT_/Audio/S_Teleport_Cue.S_Teleport_Cue" 1.0 1.0 0.0 0 0))

(event EventBeginPlay)

(event Collision|EventActorBeginOverlap
  (params (OtherActor :type Actor%20Object%20Reference)))

(event EventTick
  (params (DeltaSeconds :type Float%20%28single-precision%29)))

(fn ConstructionScript
  (Rendering|Material|SetMaterial (Variables|Default|GetCube) 0 "/Game/_MY_CONTENT_/Materials/M_HexTileBlue.M_HexTileBlue")
  (Rendering|Components|TextRender|SetText (Variables|Default|GetLevel%20Title) (Variables|Default|GetLevel)))