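; A one-shot proximity button that shifts two referenced objects and then destroys itself.
; Overlapping its Box sets a flag and enables player 0's input on the actor; leaving reverses both.
; Pressing Use plays a click sound and, while overlapped, turns the button green and teleports ObjectButton and ObjectWall by their offset vectors before the actor is destroyed.
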(event OnComponentBeginOverlap(Box)
  (params (OverlappedComponent :type Primitive%20Component%20Object%20Reference) (OtherActor :type Actor%20Object%20Reference) (OtherComp :type Primitive%20Component%20Object%20Reference) (OtherBodyIndex :type Integer) (bFromSweep :type Boolean) (SweepResult :type Hit%20Result%20Structure%20%28by%20ref%29))
  ;[1 1 1] Range
  (Variables|Default|SetIs%20Overlapped true)
  (Input|EnableInput (Game|GetPlayerController 0)))

(event OnComponentEndOverlap(Box)
  (params (OverlappedComponent :type Primitive%20Component%20Object%20Reference) (OtherActor :type Actor%20Object%20Reference) (OtherComp :type Primitive%20Component%20Object%20Reference) (OtherBodyIndex :type Integer))
  ;[1 1 1] Range
  (Variables|Default|SetIs%20Overlapped false)
  (Input|DisableInput (Game|GetPlayerController 0)))

(event Input|ActionEvents|InputActionUse
  (params (Key :type Key%20Structure :default "None"))
  (:Pressed
    (Audio|PlaySound2D "/Game/_MY_CONTENT_/Audio/S_Button_Click_Cue.S_Button_Click_Cue" 1.0 1.0 0.0 0 0)
    (if (Variables|Default|GetIs%20Overlapped)
      (Rendering|Material|SetMaterial (Variables|Default|GetButton) 0 "/Game/_MY_CONTENT_/Materials/M_Green.M_Green")
      (Transformation|SetActorLocation (Variables|Default|GetObject%20Button) (+ (Transformation|GetActorLocation (Variables|Default|GetObject%20Button)) (Variables|Default|GetVector%20Button)) false true)
      (Transformation|SetActorLocation (Variables|Default|GetObject%20Wall) (+ (Transformation|GetActorLocation (Variables|Default|GetObject%20Wall)) (Variables|Default|GetVector%20Wall)) false true)
      (Actor|DestroyActor))))

(fn ConstructionScript)