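; Pressure button that accepts a BP_Box to toggle the position of a linked Object actor.
; Each box overlap turns the button green and teleports Object by VectorOut or its negation, computed at BeginPlay, alternating via IsActivated.
; Ending an overlap turns the button red without moving Object back.
; A BP_Ball instead makes the button actor itself rise after a delay, setting its rotation, and drop on leaving.
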(event OnComponentBeginOverlap(BoxCorrect)
  (params (OverlappedComponent :type Primitive%20Component%20Object%20Reference) (OtherActor :type Actor%20Object%20Reference) (OtherComp :type Primitive%20Component%20Object%20Reference) (OtherBodyIndex :type Integer) (bFromSweep :type Boolean) (SweepResult :type Hit%20Result%20Structure%20%28by%20ref%29))
  (Variables|Default|SetIs%20Overlapped true)
  (Variables|Default|SetCorrectObject (== (Utilities|GetClass OtherActor) "/Game/_MY_CONTENT_/Blueprints/BP_Box.BP_Box_C"))
  (Variables|Default|SetIncorrectObject (== (Utilities|GetClass OtherActor) "/Game/_MY_CONTENT_/Blueprints/BP_Ball.BP_Ball_C"))
  (if (Variables|Default|GetCorrectObject)
    (if (Variables|Default|GetIs%20Overlapped)
      (Rendering|Material|SetMaterial (Variables|Default|GetButton) 0 "/Game/_MY_CONTENT_/Materials/M_Green.M_Green")
      (if (Variables|Default|GetIs%20Activated)
        (Transformation|SetActorLocation (Variables|Default|GetObject) (+ (Transformation|GetActorLocation (Variables|Default|GetObject)) (Variables|Default|GetVectorOut)) false true)
        (Variables|Default|SetIs%20Activated false)
        (else
          (Transformation|SetActorLocation (Variables|Default|GetObject) (+ (Transformation|GetActorLocation (Variables|Default|GetObject)) (Variables|Default|GetVectorIn)) false true)
          (Variables|Default|SetIs%20Activated true))))
    (elif (Variables|Default|GetIncorrectObject)
      (Utilities|FlowControl|Delay 1.0)
      (Transformation|SetActorLocationAndRotation (+ (Transformation|GetActorLocation) "0.000000, 0,20.000000") (Variables|Default|Getrotation)))))

(event OnComponentEndOverlap(BoxCorrect)
  (params (OverlappedComponent :type Primitive%20Component%20Object%20Reference) (OtherActor :type Actor%20Object%20Reference) (OtherComp :type Primitive%20Component%20Object%20Reference) (OtherBodyIndex :type Integer))
  (Variables|Default|SetIs%20Overlapped false)
  (Rendering|Material|SetMaterial (Variables|Default|GetButton) 0 "/Game/_MY_CONTENT_/Materials/M_Red.M_Red")
  (if (not (Variables|Default|GetCorrectObject))
    (if (Variables|Default|GetIncorrectObject)
      (Utilities|FlowControl|Delay 1.0)
      (Transformation|SetActorLocationAndRotation (+ (Transformation|GetActorLocation) "0.000000, 0,-20.000000") "0, 0, 0"))))

(event EventBeginPlay
  (Variables|Default|SetVectorIn (- (Variables|Default|GetVectorOut) (* (Variables|Default|GetVectorOut) 2.0))))

(fn ConstructionScript)