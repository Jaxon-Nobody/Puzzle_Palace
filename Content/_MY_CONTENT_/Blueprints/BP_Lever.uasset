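; BP_Lever is an interactable lever that toggles a referenced Object between two positions.
; Box overlap begin and end set a range flag and enable or disable input for player controller 0.
; Pressing Use plays a click sound and, in range, instantly flips the lever mesh and offsets Object by VectorIn or VectorOut.
; BeginPlay derives VectorIn as the negation of VectorOut, so each toggle reverses the last.
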(event OnComponentBeginOverlap(Box)
  (params (OverlappedComponent :type Primitive%20Component%20Object%20Reference) (OtherActor :type Actor%20Object%20Reference) (OtherComp :type Primitive%20Component%20Object%20Reference) (OtherBodyIndex :type Integer) (bFromSweep :type Boolean) (SweepResult :type Hit%20Result%20Structure%20%28by%20ref%29))
  ;[1 1 1] Range
  (Variables|Default|SetIs%20Overlapped true)
  (Input|EnableInput (Game|GetPlayerController 0)))

(event OnComponentEndOverlap(Box)
  (params (OverlappedComponent :type Primitive%20Component%20Object%20Reference) (OtherActor :type Actor%20Object%20Reference) (OtherComp :type Primitive%20Component%20Object%20Reference) (OtherBodyIndex :type Integer))
  ;[1 1 1] Range
  (Variables|Default|SetIs%20Overlapped false)
  (Input|DisableInput (Game|GetPlayerController 0)))

(event EventBeginPlay
  (Variables|Default|SetVectorIn (- (Variables|Default|GetVectorOut) (* (Variables|Default|GetVectorOut) 2.0))))

(event Input|ActionEvents|InputActionUse
  (params (Key :type Key%20Structure :default "None"))
  (bind _lever (Variables|Default|GetLever))
  (bind _lever_2 (Variables|Default|GetLever))
  (:Pressed
    (Audio|PlaySound2D "/Game/_MY_CONTENT_/Audio/S_Button_Click_Cue.S_Button_Click_Cue" 1.0 1.0 0.0 0 0)
    (if (Variables|Default|GetIs%20Overlapped)
      (if (Variables|Default|GetIs%20Activated)
        (Transformation|AddRelativeRotation _lever_2 "0, 0,-90.000000" false true)
        (Transformation|AddRelativeLocation _lever_2 "0, 0,12.000000" false false)
        (Transformation|SetActorLocation (Variables|Default|GetObject) (+ (Transformation|GetActorLocation (Variables|Default|GetObject)) (Variables|Default|GetVectorOut)) false true)
        (Variables|Default|SetIs%20Activated false)
        (else
          (Transformation|AddRelativeRotation _lever "0,0.000000,90.000000" false true)
          (Transformation|AddRelativeLocation _lever "0, 0,-12.000000" false true)
          (Transformation|SetActorLocation (Variables|Default|GetObject) (+ (Transformation|GetActorLocation (Variables|Default|GetObject)) (Variables|Default|GetVectorIn)) false true)
          (Variables|Default|SetIs%20Activated true))))))

(fn ConstructionScript)