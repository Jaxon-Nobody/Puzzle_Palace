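; BP_LevelDoor is a level door that teleports the player and marks itself as complete when its trigger box is entered.
; The construction script gives the Cube a green hex-tile material and writes the Level value to the LevelTitle text.
; Any Box overlap, with no check on the overlapping actor, moves MyPlayer to the TeleportLocation actor's position, turns the Cube red and unhides the Complete component.
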(event OnComponentBeginOverlap(Box)
  (params (OverlappedComponent :type Primitive%20Component%20Object%20Reference) (OtherActor :type Actor%20Object%20Reference) (OtherComp :type Primitive%20Component%20Object%20Reference) (OtherBodyIndex :type Integer) (bFromSweep :type Boolean) (SweepResult :type Hit%20Result%20Structure%20%28by%20ref%29))
  (Transformation|SetActorLocation (Variables|Default|GetMy%20Player) (Transformation|GetActorLocation (Variables|Default|GetTeleport%20Location)) false false)
  (Rendering|Material|SetMaterial (Variables|Default|GetCube) 0 "/Game/_MY_CONTENT_/Materials/M_HexTileRed.M_HexTileRed")
  (Development|SetHiddeninGame (Variables|Default|GetComplete) false false))

(event EventBeginPlay)

(event Collision|EventActorBeginOverlap
  (params (OtherActor :type Actor%20Object%20Reference)))

(event EventTick
  (params (DeltaSeconds :type Float%20%28single-precision%29)))

(fn ConstructionScript
  (Rendering|Material|SetMaterial (Variables|Default|GetCube) 0 "/Game/_MY_CONTENT_/Materials/M_HexTileGreen.M_HexTileGreen")
  (Rendering|Components|TextRender|SetText (Variables|Default|GetLevel%20Title) (Variables|Default|GetLevel)))